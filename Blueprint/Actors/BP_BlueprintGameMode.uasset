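; Game mode that tracks the match's win and lose conditions by counting living enemies and watching the player.
; BeginPlay scans all BP_BaseCharacter actors, binding the BP_BasePlayer's lost event and counting the rest as enemies through their OnDestroyed.
; When the count reaches zero it prints a win, calls PlayerWin and shows the results widget; losing only prints a message.
; The created widget's assignment to ResultsWidgetObject is disconnected, leaving that variable unset.
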(event EventBeginPlay
  (bind _outactors (Actor|GetAllActorsOfClass "/Game/Blueprint/Actors/BP_BaseCharacter.BP_BaseCharacter_C"))
  (for _array_element _outactors
    (bind _asbp_base_player (Utilities|Casting|CastToBP_BasePlayer _array_element)
      (:then
        (bind _output_get (Variables|Default|SetCurrentPlayer _asbp_base_player))
        (EventDispatchers|BindEventtoOnPlayerLost _output_get (EventDispatchers|CreateEvent :!event RemovePlayer)))
      (:CastFailed
        (CallFunction|AddEnemy _array_element))))
  (bind _returnvalue (Actor|GetActorOfClass (Variables|Default|GetPlayerControllerClass)))
  (bind _returnvalue_2 (UserInterface|CreateWidget (Variables|Default|GetResultsWidgetClass) _returnvalue)))

(fn ConstructionScript)

(fn RemoveEnemy
  (params (DestroyedActor :type Actor%20Object%20Reference))
  (bind _result (Math|Integer|DecrementInt (Variables|Default|GetNumberOfEnemies))
    (:%20%20
      (if (not (> _result 0))
        (Development|PrintString "YOU WIN!" true true "(R=0.000000,G=1.000000,B=0.131249,A=1.000000)" 8.0)
        (UserInterface|Viewport|AddtoViewport (Variables|Default|GetResultsWidgetObject) 0)
        (Default|PlayerWin (Variables|Default|GetCurrentPlayer))
        (Default|SetWin (Variables|Default|GetResultsWidgetObject))))))

(fn AddEnemy
  (params (EnemyActor :type Actor%20Object%20Reference))
  (Game|BindEventtoOnDestroyed EnemyActor (EventDispatchers|CreateEvent :!event RemoveEnemy))
  (Math|Integer|IncrementInt (Variables|Default|GetNumberOfEnemies)))

(fn RemovePlayer
  (Development|PrintString "YOU LOSE!" true true "(R=1.000000,G=0.000000,B=0.092665,A=1.000000)" 8.0))