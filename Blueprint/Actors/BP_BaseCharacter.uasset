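; BP_BaseCharacter is a base character Blueprint that equips a rifle and links it to the character's animation.
; BeginPlay spawns WeaponClass through a ChildActorComponent, caches it and the animation Blueprint, and binds rifle attack and reload-start events, destroying the actor if either cast fails.
; HandleHurt plays a hit animation by ratio, and CanPickupHealth returns false.
; The animation's action-ended and reload-now bindings are unconnected.
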(event EventBeginPlay
  (bind _childactorcomponent (Variables|Default|GetChildActorComponent))
  ;[1 1 1] Comment
  (|CallParentFunction)
  (ChildActorComponent|SetChildActorClass _childactorcomponent (Variables|Default|GetWeaponClass))
  (bind _asbp_base_rifle (Utilities|Casting|CastToBP_BaseRifle (Variables|/Script/Engine.ChildActorComponent|GetChildActor _childactorcomponent))
    (:then
      (Variables|Default|SetWeaponObject _asbp_base_rifle)
      (bind _asabp_character_animation (Utilities|Casting|CastToABP_CharacterAnimation (Components|SkeletalMesh|GetAnimInstance (Variables|Character|GetMesh)))
        (:then
          (Variables|Default|SetAnimationBP _asabp_character_animation)
          (EventDispatchers|BindEventtoOnRifleAttack (Variables|Default|GetWeaponObject) (EventDispatchers|CreateEvent (Variables|Default|GetAnimationBP) :!event FireAnimation))
          ;[1 1 1] come back after creating the reload animation
          (EventDispatchers|BindEventtoOnReloadStart (Variables|Default|GetWeaponObject) (EventDispatchers|CreateEvent (Variables|Default|GetAnimationBP) :!event ReloadAnimation)))
        (:CastFailed
          (Development|PrintString "We need anothe animation blueprint")
          (Actor|DestroyActor))))
    (:CastFailed
      (Development|PrintString "We need a weapon")
      (Actor|DestroyActor))))

(fn ConstructionScript)

(fn HandleHurt
  (params (Ratio :type Float%20%28double-precision%29))
  (Class|CharacterAnimation|HitAnimation (Variables|Default|GetAnimationBP) Ratio))

(fn CanPickupHealth
  (return false))