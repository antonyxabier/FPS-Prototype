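; BP_BaseAgent is a base AI agent Blueprint that attacks and reloads through a weapon object and tints its mesh from a color.
; Health and ammo handlers write to the AI controller's Blackboard, with health set full at BeginPlay and updated when hurt.
; A finished-action handler sends an AI message to the agent.
; BeginPlay binds weapon action, ammo and death-animation events, and reloads ammo.
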(event EventEnemyAttack
  (Default|Attack (Variables|Default|GetWeaponObject)))

(event EventBeginPlay
  (|CallParentFunction)
  (EventDispatchers|BindEventtoOnActionStopped (Variables|Default|GetWeaponObject) (EventDispatchers|CreateEvent :!event HandleActionFinished))
  (CallFunction|UpdateBlackboardHealth 1.0)
  (EventDispatchers|BindEventtoOnAmmoChanged (Variables|Default|GetWeaponObject) (EventDispatchers|CreateEvent :!event UpdateBlackboardAmmo))
  (Default|ReloadAmmo (Variables|Default|GetWeaponObject))
  (EventDispatchers|BindEventtoOnDeathEnded (Variables|Default|GetAnimationBP) (EventDispatchers|CreateEvent :!event K2DestroyActor)))

(event EventEnemyReload
  (Default|RequestReload (Variables|Default|GetWeaponObject)))

(fn ConstructionScript
  (|CallParentFunction)
  (Rendering|Material|SetVectorParameterValueonMaterials (Variables|Character|GetMesh) (Variables|Default|GetTintName) (Math|Conversions|ToVector(LinearColor) (Variables|Default|GetColor))))

(fn HandleActionFinished
  (Class|AIBlueprintHelperLibrary|SendAIMessage self (Variables|Default|GetMessage) 0 true))

(fn UpdateBlackboardHealth
  (params (HealthRatio :type Float%20%28double-precision%29))
  (AI|Components|Blackboard|SetValueasFloat (AI|GetBlackboard (AI|GetAIController self)) (Variables|Default|GetHealthKey) HealthRatio))

(fn HandleHurt
  (params (Ratio :type Float%20%28double-precision%29))
  (|CallParentFunction Ratio)
  (CallFunction|UpdateBlackboardHealth Ratio))

(fn UpdateBlackboardAmmo
  (params (Current :type Float%20%28double-precision%29) (Max :type Float%20%28double-precision%29))
  (AI|Components|Blackboard|SetValueasFloat (AI|GetBlackboard (AI|GetAIController self)) (Variables|Default|GetAmmoKey) Current))