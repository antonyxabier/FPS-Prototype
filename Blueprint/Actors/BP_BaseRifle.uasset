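; Base rifle actor for a parent pawn (it destroys itself without one), firing projectiles from a weapon socket and tracking ammo.
; Attack and reload share an ActionHappening lock; shots consume ammo and start a reset timer, while ReloadAmmo refills it.
; Call* functions report attack, reload, ammo and action-end changes.
; A temporary aim hack points the HUD-owning player's shots at world origin; other pawns use GetBaseAimRotation.
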(event Custom|ActionStopped
  (Variables|Default|SetActionHappening false)
  (Default|CallOnActionStopped))

(event Custom|ReloadAmmo
  (bind _maxammo (Variables|Default|GetMaxAmmo))
  (bind _output_get (Variables|Default|SetCurrentAmmo _maxammo))
  (Default|CallOnAmmoChanged _output_get _maxammo))

(event EventBeginPlay
  (|CallParentFunction)
  (bind _aspawn (Utilities|Casting|CastToPawn (Actor|GetParentActor))
    (:then
      (Variables|Default|SetParentPawn _aspawn))
    (:CastFailed
      (Development|PrintString "Owner must be a pawn")
      (Actor|DestroyActor))))

(fn ConstructionScript)

(fn Attack
  (bind _parentpawn (Variables|Default|GetParentPawn))
  (if (CallFunction|CanShoot)
    (Game|SpawnActorfromClass (Variables|Default|GetProjectileClass) (Math|Transform|MakeTransform (CallFunction|GetSource) (CallFunction|HACKDONOTEXPOSETOCODE) "1.000000,1.000000,1.000000") "Undefined" "MultiplyWithRoot" (Pawn|GetController _parentpawn) _parentpawn)
    (Variables|Default|SetActionHappening true)
    ;[1 1 1] 2 second timer before calling action stopped
    (Utilities|Time|SetTimerbyEvent (EventDispatchers|CreateEvent :!event Custom|ActionStopped) (Variables|Default|GetResetTime))
    (Default|CallOnRifleAttack)
    (CallFunction|UseAmmo)))

(fn CanShoot
  (return (and (not (Variables|Default|GetActionHappening)) (> (Variables|Default|GetCurrentAmmo) 0.0))))

(fn HACKDONOTEXPOSETOCODE
  (bind _parentpawn (Variables|Default|GetParentPawn))
  (bind _foundwidgets (Widget|GetAllWidgetsOfClass "/Game/Both/WBP_PlayerHUD.WBP_PlayerHUD_C" false))
  (if (== (Class|UserWidget|GetOwningPlayerPawn (Utilities|Array|Get(acopy) _foundwidgets)) _parentpawn)
    ;[1 1 1] this is the player override of GetBaseAimRotation
    (return (Math|Rotator|MakeRotfromX (- "" (CallFunction|GetSource))))
    (else
      (return (Pawn|GetBaseAimRotation _parentpawn)))))

(fn GetSource
  (return (Transformation|GetSocketLocation (Variables|Default|GetSkeletalMesh) (Variables|Default|GetWeaponSocketName))))

(fn UseAmmo
  (bind _output_get (Variables|Default|SetCurrentAmmo (Math|Float|Max(Float) (- (Variables|Default|GetCurrentAmmo) 1.0) 0.0)))
  (Default|CallOnAmmoChanged _output_get (Variables|Default|GetMaxAmmo)))

(fn RequestReload
  (if (not (Variables|Default|GetActionHappening))
    (Variables|Default|SetActionHappening true)
    (Default|CallOnReloadStart)))