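; BP_BasePlayer is the player pawn Blueprint, handling movement, look and weapon input.
; BeginPlay creates the HUD, binds the weapon's ammo-change event and reloads, or destroys the actor without a PlayerController.
; Axis inputs move along control yaw, while attack and reload forward to WeaponObject.
; Win and loss functions remove the HUD, health pickup is always allowed, and heal, death and fire-animation hooks are left disconnected.
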(event EventBeginPlay
  (|CallParentFunction)
  (bind _asplayer_controller (Utilities|Casting|CastToPlayerController (Pawn|GetController))
    (:then
      (bind _returnvalue (UserInterface|CreateWidget "/Game/Both/WBP_PlayerHUD.WBP_PlayerHUD_C" _asplayer_controller))
      (bind _output_get (Variables|Default|SetWBP_PlayerHUD _returnvalue))
      (UserInterface|Viewport|AddtoViewport _output_get 0)
      (EventDispatchers|BindEventtoOnAmmoChanged (Variables|Default|GetWeaponObject) (EventDispatchers|CreateEvent (Variables|Default|GetWBP_PlayerHUD) :!event SetAmmo))
      (Default|ReloadAmmo (Variables|Default|GetWeaponObject)))
    (:CastFailed
      (Development|PrintString "Failed to get controller")
      (Actor|DestroyActor))))

(event Input|ActionEvents|InputActionAttackInput
  (params (Key :type Key%20Structure))
  ;[1 1 1] Comment
  (:Pressed
    (Default|Attack (Variables|Default|GetWeaponObject))))

(event Input|ActionEvents|InputActionReload
  (params (Key :type Key%20Structure))
  (:Pressed
    (Default|RequestReload (Variables|Default|GetWeaponObject))))

(event Input|AxisEvents|InputAxisTurnRight
  (params (AxisValue :type Float%20%28single-precision%29))
  (Pawn|Input|AddControllerYawInput AxisValue))

(event Input|AxisEvents|InputAxisLookUp
  (params (AxisValue :type Float%20%28single-precision%29))
  (Pawn|Input|AddControllerPitchInput AxisValue))

(event Input|AxisEvents|InputAxisMoveForward
  (params (AxisValue :type Float%20%28single-precision%29))
  (Pawn|Input|AddMovementInput (Math|Vector|GetForwardVector (Math|Rotator|MakeRotator 0.0 0.0 (.Yaw (Math|Rotator|BreakRotator (Pawn|GetControlRotation :!class /Script/Engine.Pawn))))) AxisValue false))

(event Input|AxisEvents|InputAxisStrafe
  (params (AxisValue :type Float%20%28single-precision%29))
  (Pawn|Input|AddMovementInput (Math|Vector|GetRightVector (Math|Rotator|MakeRotator 0.0 0.0 (.Yaw (Math|Rotator|BreakRotator (Pawn|GetControlRotation :!class /Script/Engine.Pawn))))) AxisValue false))

(fn ConstructionScript
  (|CallParentFunction))

(fn CanPickupHealth
  (return true))

(fn PlayerLost
  (Default|CallOnPlayerLost)
  (Variables|/Script/Engine.PlayerController|SetbShowMouseCursor (Variables|Default|GetPlayer%20Controller) true)
  (Widget|RemovefromParent (Variables|Default|GetWBP_PlayerHUD)))

(fn PlayerWin
  (Input|DisableInput (Variables|Default|GetPlayer%20Controller))
  (Widget|RemovefromParent (Variables|Default|GetWBP_PlayerHUD)))